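; AI controller for guard NPCs that runs a guard behavior tree and reacts to perception.
; On BeginPlay it sets up the patrol blackboard and behavior tree.
; When it senses an actor not tagged Enemy, it sets the controlled character aiming and stores the player pawn in the enemy key.
; When sensing is lost, it stops shooting and clears that key, leaving aiming unchanged.
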(event OnTargetPerceptionUpdated(AIPerception)
  (params (Actor :type Actor%20Object%20Reference) (Stimulus :type AI%20Stimulus%20Structure))
  (bind _returnvalue (Pawn|GetControlledPawn))
  (bind _enemykey (Variables|Default|GetEnemyKey))
  (bind _blackboardcomp (Variables|Default|GetBlackboardComp))
  (if (not (Actor|ActorHasTag Actor "Enemy"))
    (if (.bSuccessfullySensed (Utilities|Struct|BreakAIStimulus Stimulus))
      (bind _asue4asp_hero_tpp_character_2 (Utilities|Casting|CastToUE4ASP_HeroTPP_Character2 _returnvalue))
      (Variables|/Game/Static/NPC/Behavior/UE4ASP_HeroTPP_Character2.UE4ASP_HeroTPP_Character2_C|SetAiming _asue4asp_hero_tpp_character_2 true)
      (AI|Components|Blackboard|SetValueasObject _blackboardcomp _enemykey (Game|Player|GetPlayerPawn 0))
      (else
        (bind _asue4asp_hero_tpp_character_2_2 (Utilities|Casting|CastToUE4ASP_HeroTPP_Character2 _returnvalue))
        (Variables|/Game/Static/NPC/Behavior/UE4ASP_HeroTPP_Character2.UE4ASP_HeroTPP_Character2_C|SetShooting _asue4asp_hero_tpp_character_2_2 false)
        (AI|Components|Blackboard|ClearValue _blackboardcomp _enemykey)))))

(event EventBeginPlay
  (bind _blackboardcomponent (Class|AIController|UseBlackboard "/Game/Static/NPC/AI/PatrolData.PatrolData"))
  (AI|RunBehaviorTree "/Game/Static/NPC/AI/GuardBehavior.GuardBehavior")
  (Variables|Default|SetBlackboardComp _blackboardcomponent))

(fn ConstructionScript)